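; BP_Target is a target actor in the RoboDog equipment set, with a sphere that can be shown or hidden and slides along the world X axis.
; Every tick it looks up the WBP_TableOfAnimation_Widget and mirrors its DetectTarget flag to the sphere's visibility, enabling collision only while visible.
; On BeginPlay, a timeline offsets the actor from its starting location along X, independently of that flag.
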(event `self.ReceiveTick`
  (params (DeltaSeconds :type "Float (single-precision)"))
  (bind _sphere (`self.Sphere`))
  (bind _returnvalue (`SceneComponent.IsVisible` (`self.Sphere`)))
  ;[1 1 1] Show-Hide Target
  (bind _foundwidgets (`WidgetBlueprintLibrary.GetAllWidgetsOfClass` "/Game/RoboDog/Blueprints/WBP_TableOfAnimation_Widget.WBP_TableOfAnimation_Widget_C"))
  (bind _detect_target (`/Game/RoboDog/Blueprints/WBP_TableOfAnimation_Widget.Detect Target` (`|GetArrayItem` _foundwidgets)))
  (if (!= _returnvalue _detect_target)
    _
    (else
      _))
  (`SceneComponent.SetVisibility` (`self.Sphere`) _detect_target false)
  (if _returnvalue
    (`PrimitiveComponent.SetCollisionEnabled` _sphere "QueryAndPhysics")
    (else
      (`PrimitiveComponent.SetCollisionEnabled` _sphere "NoCollision"))))

(event `self.ReceiveBeginPlay`
  (bind (_pos_x _pos_y _pos_z) (`KismetMathLibrary.BreakVector` (`self.Pos`)))
  ;[1 1 1] MoveTarget
  (set `self.Pos` (`self.K2_GetActorLocation`))
  (bind (_direction _newtrack_0) (`Timeline|Timeline_0`)
    (:`Update`
      (`self.K2_SetActorLocation` (`KismetMathLibrary.MakeVector` (- _pos_x (* (.x _newtrack_0) 900.0)) _pos_y _pos_z)))))

(fn `UserConstructionScript`)