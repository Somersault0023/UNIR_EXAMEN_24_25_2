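; BP_RoboDog is a robot dog actor that turns its turret head toward detected targets.
; A detection sphere stores any overlapping actor as the target, with the detected flag read from the DetectTarget setting on the animation table widget and cleared on overlap end.
; Each tick, while the target is valid, it passes that flag and a look-at rotation from the head's laser socket to the animation Blueprint.
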(event `self.ReceiveTick`
  (params (DeltaSeconds :type "Float (single-precision)"))
  ;[1 1 1] send data to conrol head turn
  (if (`KismetSystemLibrary.IsValid` (`self.ActorTarget`))
    (bind _asabp_robo_dog_anim_bp (cast `/Game/RoboDog/Robo_Dog/Blueprints/ABP_RoboDog_AnimBP` (`SkeletalMeshComponent.GetAnimInstance` (`self.SkeletalMesh`))))
    (set `/Game/RoboDog/Robo_Dog/Blueprints/ABP_RoboDog_AnimBP.target detected` (`self.target detected`) _asabp_robo_dog_anim_bp)
    (set `/Game/RoboDog/Robo_Dog/Blueprints/ABP_RoboDog_AnimBP.LookAt` (`KismetMathLibrary.FindLookAtRotation` (`SceneComponent.GetSocketLocation` (`self.SkeletalMesh`) "Bone_Turret_Head_LaserSocket") (`self.K2_GetActorLocation` (`self.ActorTarget`))) _asabp_robo_dog_anim_bp)))

(event `self.SphereDetectEnemy.OnComponentBeginOverlap`
  (params (OverlappedComponent :type "PrimitiveComponent Object Reference") (OtherActor :type "Actor Object Reference") (OtherComp :type "PrimitiveComponent Object Reference") (OtherBodyIndex :type Integer) (bFromSweep :type Boolean) (SweepResult :type "HitResult Structure (by ref)"))
  ;[1 1 1] detect enemy
  (bind _foundwidgets (`WidgetBlueprintLibrary.GetAllWidgetsOfClass` "/Game/RoboDog/Blueprints/WBP_TableOfAnimation_Widget.WBP_TableOfAnimation_Widget_C"))
  (set `self.target detected` (`/Game/RoboDog/Blueprints/WBP_TableOfAnimation_Widget.Detect Target` (`|GetArrayItem` _foundwidgets)))
  (set `self.ActorTarget` OtherActor))

(event `self.SphereDetectEnemy.OnComponentEndOverlap`
  (params (OverlappedComponent :type "PrimitiveComponent Object Reference") (OtherActor :type "Actor Object Reference") (OtherComp :type "PrimitiveComponent Object Reference") (OtherBodyIndex :type Integer))
  ;[1 1 1] detect enemy
  (set `self.target detected` false))

(fn `UserConstructionScript`)